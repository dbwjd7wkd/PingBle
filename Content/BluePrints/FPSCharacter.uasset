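; First-person player character Blueprint that adds a reticle widget at start and handles camera-relative movement and hitscan shooting.
; Left click line-traces along the camera up to weapon range, turns on ragdoll physics for a hit Ue4ASP_Character, and calls a fixed impulse on Mesh at the hit bone.
; A DoOnce and FlipFlop alternate two muzzle flashes per click, both hidden on release.
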(event `self.ReceiveBeginPlay`
  ;[1 1 1] UI
  (bind _returnvalue (`|CreateWidget` "/Game/UI/Recticle.Recticle_C" (`GameplayStatics.GetPlayerController` 0)))
  (`UserWidget.AddToViewport` _returnvalue 0))

(event `InputAxis|MoveRight`
  (params (AxisValue :type "Float (single-precision)"))
  ;[1 1 1] movement
  (`self.AddMovementInput` (`SceneComponent.GetRightVector` (`self.Camera`)) AxisValue))

(event `InputAxis|MoveForward`
  (params (AxisValue :type "Float (single-precision)"))
  ;[1 1 1] movement
  (`self.AddMovementInput` (`SceneComponent.GetForwardVector` (`self.Camera`)) AxisValue))

(event `Key|LeftMouseButton`
  (params (Key :type "Key Structure"))
  (bind _camera (`self.Camera`))
  (bind _returnvalue (`SceneComponent.K2_GetComponentLocation` _camera))
  (:`Pressed`
    (`|ExecutionSequence`
      (:`then_0`
        (bind _outhit (`KismetSystemLibrary.LineTraceSingle` _returnvalue (+ _returnvalue (* (`SceneComponent.GetForwardVector` _camera) (`self.WeaponRange`))) "TraceTypeQuery1"))
        (bind (_bblockinghit _binitialoverlap _time _distance _location _impactpoint _normal _impactnormal _physmat _hitactor _hitcomponent _hitbonename) (`GameplayStatics.BreakHitResult` _outhit))
        (bind _asue_4asp_character (cast `/Game/AnimStarterPack/Ue4ASP_Character` _hitactor))
        (`PrimitiveComponent.SetSimulatePhysics` (`Character.Mesh` _asue_4asp_character) true)
        (`PrimitiveComponent.AddImpulse` (`self.Mesh`) (1000.0 1000.0 0.0) _hitbonename false))
      (:`then_1`
        ;[1 1 1] FX & Audio
        (`/Engine/EditorBlueprintResources/StandardMacros.DoOnce` false :!label _label
          (:`Completed`
            (`/Engine/EditorBlueprintResources/StandardMacros.FlipFlop`
              (:`A`
                (`SceneComponent.SetVisibility` (`self.MuzzleFlash`) true false))
              (:`B`
                (`SceneComponent.SetVisibility` (`self.muzzle2`) true false))))))))
  (:`Released`
    (`SceneComponent.SetVisibility` (`self.MuzzleFlash`) false false)
    (`SceneComponent.SetVisibility` (`self.muzzle2`) false false)
    (goto _label :!via `Reset`)))

(fn `UserConstructionScript`)