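; BP_EnemyProjectile is a projectile that flies toward where the first-person character stood when it spawned.
; BeginPlay finds the FirstPersonCharacter, stores a one-time direction through FindDirection (world +X if none is valid) and sets a short lifespan.
; Tick moves it manually with a swept SetActorLocation, without homing.
; Box overlaps with anything except BP_Enemy destroy it, and no damage is applied here.
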(event `self.ReceiveBeginPlay`
  (bind _returnvalue (`GameplayStatics.GetActorOfClass` "/Game/FirstPersonCPP/Blueprints/FirstPersonCharacter.FirstPersonCharacter_C"))
  (set `self.Target` _returnvalue)
  (`self.FindDirection`)
  (`self.SetLifeSpan` 2.0))

(event `self.ReceiveTick`
  (params (DeltaSeconds :type "Float (single-precision)"))
  ;[1 1 1] 이동하기
  ;;[1 1 1] P
  (`self.K2_SetActorLocation` (+ (* (* (`KismetMathLibrary.Normal` (`self.Direction`)) (`self.Speed`)) DeltaSeconds) (`self.K2_GetActorLocation`)) true))

(event `self.Box.OnComponentBeginOverlap`
  (params (OverlappedComponent :type "PrimitiveComponent Object Reference") (OtherActor :type "Actor Object Reference") (OtherComp :type "PrimitiveComponent Object Reference") (OtherBodyIndex :type Integer) (bFromSweep :type Boolean) (SweepResult :type "HitResult Structure (by ref)"))
  (cast `/Game/AI/BP_Enemy` OtherActor
    (:`CastFailed`
      (`self.K2_DestroyActor`))))

(fn `FindDirection`
  (bind _target (`self.target`))
  (`/Engine/EditorBlueprintResources/StandardMacros.IsValid` _target
    (:`Is Valid`
      (set `self.Direction` (- (`self.K2_GetActorLocation` _target) (`self.K2_GetActorLocation`))))
    (:`Is Not Valid`
      (set `self.Direction` (1.0 0.0 0.0)))))

(fn `UserConstructionScript`)