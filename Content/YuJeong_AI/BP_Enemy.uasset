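; BP_Enemy is an enemy with a widget energy bar that either deflects or absorbs incoming FirstPersonProjectile hits.
; On capsule hit, about 70% of projectiles have their velocity reversed while the enemy turns to the player, animates and flashes a muzzle effect.
; The rest are destroyed and reduce energy.
; At zero energy it shows the win screen and cursor, spawns BP_Enemy_Death to play the death animation, and destroys itself.
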(event `self.ReceiveBeginPlay`
  ;[1 1 1] 에너지바표시하기
  (bind _asenergybar (cast `/Game/UI/Energybar` (`WidgetComponent.GetUserWidgetObject` (`self.EnergybarWidget`))))
  (bind _output_get (set `self.Energybar_UI` _asenergybar))
  (bind _output_get_2 (set `/Game/UI/Energybar.EnergyPercent` (/ (`self.Energy`) (`self.Init_Energy`)) _output_get))
  (`/Game/UI/Energybar.SetEnergyPercent` (`self.Energybar_UI`) _output_get_2))

(event `self.CapsuleComponent.OnComponentHit`
  (params (HitComponent :type "PrimitiveComponent Object Reference") (OtherActor :type "Actor Object Reference") (OtherComp :type "PrimitiveComponent Object Reference") (NormalImpulse :type "Vector Structure") (Hit :type "HitResult Structure (by ref)"))
  ;[1 1 1] 에너지줄이기, 70%는 Player 공격 튕겨내고 30%는 들어온 발사체 없애기
  (bind _asfirst_person_projectile (cast `/Game/FirstPersonBP/Blueprints/FirstPersonProjectile` OtherActor))
  (if (> (`KismetMathLibrary.RandomIntegerInRange` 1 100) 30)
    (bind _projectilemovement (`/Game/FirstPersonBP/Blueprints/FirstPersonProjectile.ProjectileMovement` _asfirst_person_projectile))
    ;;[1 1 1] 공격 튕겨내기
    (set `MovementComponent.Velocity` (* (`MovementComponent.Velocity` _projectilemovement) -1) _projectilemovement)
    (`self.RoationToPlayer`)
    (`SkeletalMeshComponent.PlayAnimation` (`self.Mesh`) "/Game/YuJeong_AI/Animations/Using/Enemy_Ability_Deflicting.Enemy_Ability_Deflicting" false)
    ;[1 1 1] 불꽃생성
    (`/Engine/EditorBlueprintResources/StandardMacros.DoOnce` false :!label _label
      (:`Completed`
        (`SceneComponent.SetVisibility` (`self.MuzzleFlash`) true false)
        (`KismetSystemLibrary.Delay` 1.0)
        (`SceneComponent.SetVisibility` (`self.MuzzleFlash`) false false)
        (goto _label :!via `Reset`)))
    (else
      (`self.K2_DestroyActor` OtherActor)
      ;[1 1 1] 공격을 맞으면 에너지가 줄어들고, 0 보다 작아지면 죽는다.
      (`self.CutEnergy`)
      (`self.IsDying`))))

(fn `CutEnergy`
  ;[1 1 1] 공격을 맞으면 에너지가 줄어들고, 에너지가 0이 되면 적이 없어진다.
  (set `self.Energy` (- (`self.Energy`) (`self.Damage`)))
  (set `/Game/UI/Energybar.EnergyPercent` (/ (`self.Energy`) (`self.Init_Energy`)) (`self.Energybar_UI`)))

(fn `IsDying`
  ;[1 1 1] 에너지가 0이하가 되면 죽음
  (if (<= (`self.Energy`) 0.0)
    ;[1 1 1] 죽었을 때 UI 띄우기
    (bind _returnvalue (`|CreateWidget` "/Game/UI/WBP_Gameover_Win.WBP_Gameover_Win_C"))
    (`UserWidget.AddToViewport` _returnvalue 0)
    ;[1 1 1] 마우스 보이게 하기
    (set `PlayerController.bShowMouseCursor` true (`GameplayStatics.GetPlayerController` 0))
    ;[1 1 1] 죽었을 때 애니메이션 재생 (새로운 액터 spawn해서 거기에 애니메이션 재생)
    (bind _returnvalue_2 (`|SpawnActorFromClass` "/Game/YuJeong_AI/BP_Enemy_Death.BP_Enemy_Death_C" (`self.GetTransform`) "AlwaysSpawn" "OverrideRootScale" null null))
    (`SkeletalMeshComponent.PlayAnimation` (`Character.Mesh` _returnvalue_2) "/Game/YuJeong_AI/Animations/Using/Enemy_Death_Forward.Enemy_Death_Forward" false)
    (`self.K2_DestroyActor`)))

(fn `RoationToPlayer`
  ;[1 1 1] player 얼굴을 향해 몸 돌리기
  (`SceneComponent.K2_SetWorldRotation` (`self.CapsuleComponent`) (`KismetMathLibrary.FindLookAtRotation` (`SceneComponent.K2_GetComponentLocation` (`self.CapsuleComponent`)) (`self.K2_GetActorLocation` (`GameplayStatics.GetPlayerCharacter` 0))) false false))

(fn `UserConstructionScript`)