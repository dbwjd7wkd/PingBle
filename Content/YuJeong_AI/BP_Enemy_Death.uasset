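; BP_Enemy_Death is an actor that, judging by its name, presents an enemy death as a slow-motion victory moment.
; Shortly after BeginPlay, it plays the Overwatch victory BGM and slows global time to one tenth, with no restore in this Blueprint.
; Each Tick moves it along its normalized Direction by Speed and delta time using a swept SetActorLocation, so the motion follows the time dilation.
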(event `self.ReceiveBeginPlay`
  ;[1 1 1] 승리 노래 틀기
  (`KismetSystemLibrary.Delay` 0.2)
  (`GameplayStatics.PlaySound2D` "/Game/Sounds/Overwatch_Victory_BGM_Cue.Overwatch_Victory_BGM_Cue" 1.0 1.0 0.0 null null)
  ;[1 1 1] 시간 10배 느리게 하기
  (`GameplayStatics.SetGlobalTimeDilation` 0.1))

(event `self.ReceiveActorBeginOverlap`
  (params (OtherActor :type "Actor Object Reference")))

(event `self.ReceiveTick`
  (params (DeltaSeconds :type "Float (single-precision)"))
  ;[1 1 1] 이동하기
  ;;[1 1 1] P
  (`self.K2_SetActorLocation` (+ (* (* (`KismetMathLibrary.Normal` (`self.Direction`)) (`self.Speed`)) DeltaSeconds) (`self.K2_GetActorLocation`)) true))

(fn `UserConstructionScript`)